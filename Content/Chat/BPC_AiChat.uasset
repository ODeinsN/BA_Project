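; BPC_AiChat is a component that opens and closes dialog chat between the player and an AI character.
; OpenChat and CloseChat swap input mapping context, HUD and mouse cursor, closing the previous HUD via BPI_ClosableHud, then fire opened or closed notifications.
; On open, the partner's history fills HUD_Chat, and its models and name configure NeoLlama before its information collection loads into a database.
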(event Input|EnhancedActionEvents|EnhancedInputActionIA_CloseChat
  (params (ActionValue :type Boolean) (ElapsedSeconds :type Float%20%28double-precision%29) (TriggeredSeconds :type Float%20%28double-precision%29) (InputAction :type Input%20Action%20Object%20Reference :default "/Game/Chat/Inputs/InputActions/IA_CloseChat.IA_CloseChat"))
  (if (Variables|Default|GetChatIsActive)
    (CallFunction|CloseChat)))

(fn OpenChat
  (params (ChatPartner :type BPI%20Ai%20Chat%20Partner%20Interface))
  (bind _returnvalue (Game|GetPlayerController 0))
  (bind _returnvalue_2 (Game|GetPlayerController 0))
  (bind _returnvalue_3 (HUD|GetHUD _returnvalue_2))
  (bind _returnvalue_4 (PlayerController|LocalPlayerSubsystems|GetEnhancedInputLocalPlayerSubsystem _returnvalue))
  (Variables|Default|SetCurrentChatPartner ChatPartner)
  (Utilities|FlowControl|Sequence
    (:then_0
      ;[0.05 0.05 0.05] Change to ChatInputMapping Context
      (Utilities|IsValid _returnvalue_4
        (:Is%20Valid
          (Input|RemoveMappingContext _returnvalue_4 "/Game/Example/FirstPerson/Input/IMC_Default.IMC_Default" "(bIgnoreAllPressedKeysUntilRelease=True,bForceImmediately=False,bNotifyUserSettings=False)")
          (Input|AddMappingContext _returnvalue_4 "/Game/Chat/Inputs/IMC_ChatDialog.IMC_ChatDialog" 0 "(bIgnoreAllPressedKeysUntilRelease=True,bForceImmediately=False,bNotifyUserSettings=False)")
          (Variables|Default|SetChatIsActive true))))
    (:then_1
      ;[0.05 0.05 0.05] close old HUD
      (Utilities|ClosePreviousHUD))
    (:then_2
      ;[0.05 0.05 0.05] open Chat HUD
      (Class|PlayerController|ClientSetHUD (Game|GetPlayerController 0) "/Game/Chat/UI/HUD_Chat.HUD_Chat_C")
      (Class|BPIClosableHud|OpenHUD(Message) _returnvalue_3)
      (bind _ashud_chat (Utilities|Casting|CastToHUD_Chat _returnvalue_3))
      (Variables|Default|SetChatHUD _ashud_chat))
    (:then_3
      ;[0.05 0.05 0.05] Enable mouse cursor
      (Variables|/Script/Engine.PlayerController|SetbShowMouseCursor (Game|GetPlayerController 0) true))
    (:then_4
      (Utilities|FlowControl|Sequence
        (:then_0
          ;[0.05 0.05 0.05] Load Message History
          (bind _messages (Default|GetMessageHistory (Variables|Default|GetCurrentChatPartner)))
          (Class|BPIChatHUD|LoadMessages(Message) (Variables|Default|GetChatHUD) _messages))
        (:then_1
          ;[0.05 0.05 0.05] setup llama component
          (Utilities|FlowControl|Sequence
            (:then_0
              (bind _model (Default|GetCypherModel (Variables|Default|GetCurrentChatPartner)))
              (Variables|/Game/Llama/BPC_NeoLlama.BPC_NeoLlama_C|SetCypherModel (Variables|Default|GetNeoLlama) _model))
            (:then_1
              (bind _model_2 (Default|GetDialogModel (Variables|Default|GetCurrentChatPartner)))
              (Variables|/Game/Llama/BPC_NeoLlama.BPC_NeoLlama_C|SetDialogModel (Variables|Default|GetNeoLlama) _model_2))
            (:then_2
              (bind _name (Default|GetCharacterName (Variables|Default|GetCurrentChatPartner)))
              (Variables|/Game/Llama/BPC_NeoLlama.BPC_NeoLlama_C|SetCharacterName (Variables|Default|GetNeoLlama) _name))
            (:then_3
              (Default|Init (Variables|Default|GetNeoLlama))
              (bind _informationcollection (Default|GetInformationCollection (Variables|Default|GetCurrentChatPartner)))
              (Class|IDSInformationCollection|LoadIntoDb _informationcollection))))))
    (:then_5
      (Default|CallOnChatOpened))))

(fn CloseChat
  (bind _returnvalue (Game|GetPlayerController 0))
  (bind _returnvalue_2 (Game|GetPlayerController 0))
  (bind _returnvalue_3 (PlayerController|LocalPlayerSubsystems|GetEnhancedInputLocalPlayerSubsystem _returnvalue))
  (Utilities|FlowControl|Sequence
    (:then_0
      ;[0.05 0.05 0.05] Switch to default MappingContext
      (Utilities|IsValid _returnvalue_3
        (:Is%20Valid
          (Input|RemoveMappingContext _returnvalue_3 "/Game/Chat/Inputs/IMC_ChatDialog.IMC_ChatDialog" "(bIgnoreAllPressedKeysUntilRelease=True,bForceImmediately=False,bNotifyUserSettings=False)")
          (Input|AddMappingContext _returnvalue_3 "/Game/Example/FirstPerson/Input/IMC_Default.IMC_Default" 0 "(bIgnoreAllPressedKeysUntilRelease=True,bForceImmediately=False,bNotifyUserSettings=False)")
          (Variables|Default|SetChatIsActive false))))
    (:then_1
      ;[0.05 0.05 0.05] close Chat HUD
      (Utilities|ClosePreviousHUD))
    (:then_2
      ;[0.05 0.05 0.05] open FPS HUD
      (Class|PlayerController|ClientSetHUD (Game|GetPlayerController 0) "/Game/UI/HUD_FPS.HUD_FPS_C"))
    (:then_3
      ;[0.05 0.05 0.05] disable mouse cursor
      (Variables|/Script/Engine.PlayerController|SetbShowMouseCursor _returnvalue_2 false)
      (Input|SetInputModeGameOnly _returnvalue_2 false))
    (:then_4
      (Default|CallOnChatClosed))))

(fn AddMessage
  (params (Message :type F%20Chat%20Message%20Structure))
  (Default|AddMessage (Variables|Default|GetChatHUD) Message))