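; BP_ChatTestActor is an interactable test actor that acts as a conversation partner for the AI chat system.
; On StartInteract it finds BPC_AiChat on the player pawn and calls OpenChat with itself as the target.
; Getter functions expose its interaction hint, dialog model, cypher model, information collection and message history.
; Its character name comes from the information collection, with an empty string when that is invalid.
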(event EventStartInteract
  (bind _returnvalue (Game|Player|GetPlayerPawn 0))
  (Utilities|IsValid _returnvalue
    (:Is%20Valid
      (Default|OpenChat (Actor|GetComponentbyClass _returnvalue "/Game/Chat/BPC_AiChat.BPC_AiChat_C") self))))

(fn ConstructionScript)

(fn CanInteract
  (return (Variables|Default|GetInteractionHint)))

(fn GetCharacterName
  (bind _informationcollection (CallFunction|GetInformationCollection))
  (Utilities|IsValid _informationcollection
    (:Is%20Valid
      (return (Utilities|String|ToString(Text) (Class|IDSInformationCollection|GetOwnCharacterName _informationcollection))))
    (:Is%20Not%20Valid
      (return ""))))

(fn GetCypherModel
  (return (Variables|Default|GetCypherModel)))

(fn GetDialogModel
  (return (Variables|Default|GetDialogModel)))

(fn GetInformationCollection
  (return (Variables|Default|GetInformationCollection)))

(fn GetMessageHistory
  (return (Variables|Default|GetMessageHistory)))