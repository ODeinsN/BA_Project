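; NPC dialogue component that pairs two LLMs with a Neo4j graph database serving as the character's memory.
; The Cypher model, primed with the database schema, turns queued messages into queries and is re-prompted on query errors.
; Query results enter the roleplay dialog model as a think block, and its partial and full replies are passed on.
; New messages stop running generations, with cancellation state used to discard stale responses.
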(event Custom|StartDialogPromptingEvent
  (Utilities|GenerateDialogResponse))

(event Custom|Init
  (|BindEvents)
  (Utilities|LoadCypherModel)
  (Utilities|LoadDialogModel))

(event Custom|AddMessage
  (params (Message :type String))
  (Utilities|Array|Add (Variables|Default|GetCypherMessageQueue) Message)
  (Utilities|Array|Add (Variables|Default|GetDialogMessageQueue) Message)
  (Utilities|StopGeneration))

(event Custom|ProcessMessages
  (Utilities|ProcessMessageQueue))

(event Custom|OnCypherModelResponseGenerated
  (params (Response :type String))
  (bind _cyphergenerationcancellations (Variables|Default|GetCypherGenerationCancellations))
  (Variables|Default|SetCypherGenerationRunning false)
  (if (== _cyphergenerationcancellations 0)
    (|HandleCypherPrompt Response)
    (else
      (Math|Integer|DecrementInt _cyphergenerationcancellations
        (:%20%20
          (Development|PrintString "Canceled cypher response"))))))

(event Custom|On%20Cypher%20Model%20loaded
  (params (ModelName :type String))
  (Utilities|CypherLoadHandler
    (:PostPreload
      (if (not (Variables|Default|GetCypherSystemPromptInjected))
        (CallFunction|GetDbSchema (Variables|Default|GetNeo4jSchemaReceiver))))))

(event Custom|OnDialogModelLoaded
  (params (ModelName :type String))
  (Utilities|DialogLoadHandler))

(event Custom|On%20Dialog%20Model%20Partial%20Response%20Generated
  (params (Partial :type String))
  (if (not (Variables|Default|GetDialogGenerationCancelled))
    (Default|CallPartialResponseGenerated Partial)))

(event Custom|On%20Dialog%20Model%20Full%20Response%20Generated
  (params (Response :type String))
  (Variables|Default|SetDialogGenerationRunning false)
  (if (not (Variables|Default|GetDialogGenerationCancelled))
    (Default|CallFullResponseGenerated Response)
    (else
      (Variables|Default|SetDialogGenerationCancelled false))))

(event Custom|On%20Data%20Query%20Response
  (params (Response%20Object :type BP%20BA%20Graph%20DB%20Response%20Object%20Reference) (RawResponse :type String))
  (bind _error_text (Default|GetErrors Response%20Object))
  (bind _cyphergenerationcancellations (Variables|Default|GetCypherGenerationCancellations))
  (if (== _cyphergenerationcancellations 0)
    (if (or (Utilities|Array|IsEmpty (Variables|Default|GetQuery%20Cache)) (Utilities|Enum|Equal(Enum) (Utilities|Text|FormatText "No errors") _error_text))
      (Variables|Default|SetResponse%20Cache (CallFunction|ResponsetoString Response%20Object))
      (Variables|Default|SetResponseReady true)
      (CallFunction|StartDialogPromptingEvent)
      (else
        (Development|PrintText (Utilities|Text|FormatText "An error occured: {error} 
Regenerating Query" _error_text))
        (Class|LlamaComponent|InsertTemplatedPrompt (Variables|Default|GetCypherModel) (Utilities|String|ToString(Text) (Utilities|Text|FormatText "An Error has occured with your cypher query.  
Analyse the cause of the error,  surround the new query string with <query> ... </query>, don't include newline or non ascii characters and fix the error: 
 
{error}" _error_text)) "User" false true)))
    (else
      (Math|Integer|DecrementInt _cyphergenerationcancellations))))

(event Custom|On%20Db%20Schema%20Response
  (params (Response%20Object :type BP%20BA%20Graph%20DB%20Response%20Object%20Reference) (RawResponse :type String))
  (bind _cyphermodel (Variables|Default|GetCypherModel)
    (:then
      (Class|LlamaComponent|InsertTemplatedPrompt _cyphermodel (Utilities|String|ToString(Text) (Utilities|Text|FormatText "Task:Generate Cypher statement to query a graph database. 
    Instructions: 
    Use only the provided relationship types and properties in the schema. 
The queries are strictly case sensitive. Always make sure that the Casing of properties matches the schema!!! 
Property names are always in camelCase! 
 
schema: 
{schema} 
 
    Do not use any other relationship types or properties that are not provided. .  
    Note: Do not include any explanations or apologies in your responses! 
ALWAYS prefix the query with <query> and suffix it with </query>!! 
    Do not respond to any questions that might ask anything else than for you to construct a Cypher statement. 
If you are being directly addressed, then the question is about your character called: \"{name}\"ALWAYS limit your result set to a maximum of 10! 
Use recursive Queries if neccessary. 
NEVER query for all possible nodes. 
All must be in a single line. Don't include Next line or end of line characters! 
ALWAYS use CONTAINS for string type properties and comparisons and if used don't include them in the Node bracked eg. (p:Person) where p.name contains 'something' instead of (p:Person `{name: 'something'`}) 
DO NOT INCLUDE ANY TEXT EXCEPT THE GENERATED CYPHER STATEMENT! 
Reduce your thinking process to a maximum of 2 sentences or 30 tokens! 
Ignore the NodeId property! 
ONLY use ASCII characters for your Query!! 
If your are defining an alias, always use 'AS'. 
Write all Cypher reserved keywords like: AS, MATCHES, RETURN in upper case. 
If the schema can't answer the qustion reply the following: 
<query>return []</query> 
DON'T query for unnecessary information! 
 
    Examples: Here are a few examples of generated Cypher statements for particular questions: 
    # How many people played in Top Gun? 
    MATCH (m:Movie)<-[:ACTED_IN]-() RETURN count(*)  AS numberOfActors WHERE m.title CONTAINS 'Top Gun' 
 
# Have you anything about Walter? 
MATCH (p:Person)-[]-() as relations WHERE p.name CONTAINS 'Walter' return relations 
" RawResponse (Variables|Default|GetCharacterName))) "System" false false)
      (Variables|Default|SetCypherSystemPromptInjected true)
      (CallFunction|ProcessMessages))
    (:else)))